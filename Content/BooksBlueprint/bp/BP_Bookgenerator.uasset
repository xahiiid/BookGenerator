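; Book generator Blueprint that builds a row of randomly chosen meshes along local X in its construction script, with no active runtime logic.
; A seeded random stream picks each mesh from the pool and sets its pitch, scaled by a rotation setting.
; Tilt direction alternates per book to tighten gaps, while component bounds and pivot offsets, measured on world X, accumulate each position plus configurable spacing.
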(fn `UserConstructionScript`
  (bind (_origin _boxextent) (`KismetSystemLibrary.GetComponentBounds` (`self.AddedMesh`)))
  (bind (_origin_2 _boxextent_2) (`KismetSystemLibrary.GetComponentBounds` (`self.AddedMesh`)))
  (bind _returnvalue_x (`KismetMathLibrary.BreakVector` (`SceneComponent.K2_GetComponentLocation` (`self.AddedMesh`))))
  (bind _returnvalue_x_2 (`KismetMathLibrary.BreakVector` (`SceneComponent.K2_GetComponentLocation` (`self.AddedMesh`))))
  (for _ (range (+ (`self.Number of mesh`) 1))
    ;[1 1 1 1 24] Set Rotation Direction based on evenness of index.
    ; Thanks to this we lower the spacing if small book is next to big book
    (set `self.RotationDirection` (* (`self.RotationDirection`) -1.0))
    ;[1 1 1 1 24] Add Static Mesh Component and set its mesh from Meshes Pool at random
    (bind _returnvalue (`AddComponent|NODE_AddStaticMeshComponent-5` :`RelativeTransform` (`KismetMathLibrary.MakeTransform` (0.0 0.0 0.0) (`KismetMathLibrary.MakeRotator` 0.0 (* (`KismetMathLibrary.RandomFloatFromStream` (`self.Seed`)) (`self.RotationDirection`) (`self.rotating`))))))
    (bind _output_get (set `self.AddedMesh` _returnvalue))
    (`StaticMeshComponent.SetStaticMesh` _output_get (`KismetArrayLibrary.Array_RandomFromStream` (`self.New Mesh`) (`self.Seed`)))
    ;[1 1 1 1 24] Recalculate position
    (set `self.NewMeshPosition` (+ (- _returnvalue_x (.x _origin)) (.x _boxextent) (`self.NewMeshPosition`)))
    (`SceneComponent.K2_SetRelativeLocation` (`self.AddedMesh`) (`KismetMathLibrary.MakeVector` (`self.NewMeshPosition`)) false false)
    ;[1 1 1 1 24] Recalculate position
    (set `self.NewMeshPosition` (+ (* (- _returnvalue_x_2 (.x _origin_2)) -1.0) (.x _boxextent_2) (`self.NewMeshPosition`) (`self.sapcing`)))))